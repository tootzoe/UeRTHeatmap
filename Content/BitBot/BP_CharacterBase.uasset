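; BP_CharacterBase is a base character Blueprint that supplies player input to the Mover movement system.
; ProduceInput clamps the IA_Move axes, rotates them by control rotation and sets the result as directional input on a character default inputs struct.
; That struct also carries control rotation, the IA_Jump press and a zero orientation intent, and is returned in a Mover input command context.
; The event graph and construction script are empty.
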(event EventBeginPlay)

(event Collision|EventActorBeginOverlap
  (params (OtherActor :type Actor%20Object%20Reference)))

(event EventTick
  (params (DeltaSeconds :type Float%20%28single-precision%29)))

(fn ConstructionScript)

(fn ProduceInput
  (params (SimTimeMs :type Integer))
  (bind _returnvalue (Pawn|GetControlRotation :!class /Script/Engine.Pawn))
  (bind _returnvalue_2 (Input|EnhancedActionValues|GetIA_Move))
  (bind _returnvalue_3 (Input|EnhancedActionValues|GetIA_Jump))
  (bind _moverdatacollection (Utilities|Struct|MakeMoverDataCollection))
  (bind _returnvalue_4 (Class|KismetMathLibrary|ClampAxes2D _returnvalue_2 -1.0 1.0))
  (bind _characterdefaultinputs (Utilities|Struct|MakeCharacterDefaultInputs "0.000000,0.000000,0.000000" _returnvalue "None" false 0 "None" _returnvalue_3))
  (Class|MoverDataModelBlueprintLibrary|SetDirectionalInput _characterdefaultinputs (Math|Vector|RotateVector (Math|Vector|MakeVector (.y _returnvalue_4) (.x _returnvalue_4) 0.0) _returnvalue))
  (Class|MoverDataCollectionLibrary|AddDatatoCollection _moverdatacollection _characterdefaultinputs)
  (return (Utilities|Struct|MakeMoverInputCmdContext _moverdatacollection)))