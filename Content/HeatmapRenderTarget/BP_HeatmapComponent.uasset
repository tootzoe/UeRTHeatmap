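; Actor component that paints a heatmap into a render target along the path of its owning actor.
; It ticks at a fixed DrawRate, line tracing downward through the owner on the Heatmap trace channel.
; The hit UV, which requires the "Support UV from Hit Results" project setting, positions a brush material drawn onto the render target canvas, offset by half the brush size.
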(event Custom|DrawToRenderTarget
  (bind _returnvalue (Components|GetOwner))
  (bind _brushsize (Variables|Default|GetBrushSize))
  (bind _returnvalue_2 (Transformation|GetActorLocation _returnvalue))
  (bind (_canvas _size _context) (Rendering|BeginDrawCanvastoRenderTarget (Variables|Default|GetRenderTarget)))
  (bind _outhit (Collision|LineTraceByChannel (+ _returnvalue_2 "0.000000,0.000000,50.000000") (+ _returnvalue_2 "0.000000,0.000000,-300.000000") "TraceTypeQuery3" true 0 "None")) ; Trace just for meshes that use the Heatmap trace channel
  (Canvas|DrawMaterial :self _canvas :RenderMaterial "/Game/HeatmapRenderTarget/M_RenderTargetBrush.M_RenderTargetBrush" :ScreenPosition (- (* _size (.UV (Class|GameplayStatics|FindCollisionUV _outhit))) (/ _brushsize 2.0)) :ScreenSize (Math|Conversions|ToVector2D(Vector) _brushsize) :CoordinateSize "(X=1.000000,Y=1.000000)" :PivotPoint "(X=0.500000,Y=0.500000)") ; Apply brush material to the render target\nat the same UV location as the Line Trace\nHit UVs
  (Rendering|EndDrawCanvastoRenderTarget _context))

(event EventBeginPlay
  (Class|ActorComponent|SetComponentTickInterval (/ 1.0 (Variables|Default|GetDrawRate))) ; This will make sure the tick and the \nrender target drawing happens on a \nfixed time scale instead of whatever \nthe current frame rate is.
)

(event EventTick
  (params (DeltaSeconds :type Float%20%28single-precision%29))
  (CallFunction|DrawtoRenderTarget))